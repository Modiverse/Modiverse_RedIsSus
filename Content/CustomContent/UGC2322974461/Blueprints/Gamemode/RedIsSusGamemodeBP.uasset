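; Game mode for Red Is Sus, an impostor-versus-crewmate social deduction game that manages players and a lobby leader.
; A one-second timer drives a game/round state machine from lobby, through settings-triggered start, into active rounds.
; Rounds shuffle players into roles, deal crewmates random tasks by type quota, and teleport everyone to tagged spawn points.
; Task completion is a stub, and win checks on alive counts only print results.
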(event `self.GameModeActivated`
  (`KismetSystemLibrary.PrintString` "Gamemode activated" true true (struct :`G` 0.66 :`B` 1.0 :`A` 1.0) 10.0)
  ;[1 1 1] Always spawn our players as spectators initially, we will make them full players later
  (`self.SetJoiningPlayersParameters` (make `KJModGameModeProxyPlayerJoinParameters` true 0.0 false 5.0 0.0))
  (`self.SwitchToNewState` "NewEnumerator0")
  (`KismetSystemLibrary.K2_SetTimer` null "CheckState" 1.0 true)
  (`self.CreateSpawnPointList`))

(event `PlayerCompletedTaskServer`
  (params (TaskId :type String) (Player :type "/Game/CustomContent/UGC2322974461/Blueprints/Player/RedIsSusPlayerBP Object Reference"))
  (`KismetSystemLibrary.PrintString` "this is where we mark the task as completed for the player")
  (`KismetSystemLibrary.PrintString` "it is also where we update the taskbar (if we should) for all players."))

(event `SetSettings`
  (params (Settings :type "/Game/CustomContent/UGC2322974461/Blueprints/Settings/SettingsStruct Structure"))
  (set `self.Settings` Settings)
  (`self.SwitchToNewState` "NewEnumerator6"))

(event `InitalizeTasks`
  (`KismetArrayLibrary.Array_Clear` (`self.Tasks`))
  (bind _outactors (`GameplayStatics.GetAllActorsOfClass` "/Game/CustomContent/UGC2322974461/Blueprints/Tasks/BaseTask/BaseTaskBP.BaseTaskBP_C"))
  (for (_array_element _array_index) _outactors
    (`KismetArrayLibrary.Array_Add` (`self.Tasks`) (make `/Game/CustomContent/UGC2322974461/Blueprints/Tasks/BaseTask/TaskStruct` _array_index (`/Game/CustomContent/UGC2322974461/Blueprints/Tasks/BaseTask/BaseTaskBP.Title` _array_element) (`/Game/CustomContent/UGC2322974461/Blueprints/Tasks/BaseTask/BaseTaskBP.CommonTask` _array_element) (`/Game/CustomContent/UGC2322974461/Blueprints/Tasks/BaseTask/BaseTaskBP.Length` _array_element) _array_element))
    (set `/Game/CustomContent/UGC2322974461/Blueprints/Tasks/BaseTask/BaseTaskBP.GamemodeBP` self _array_element)))

(fn `CheckState`
  (switch `/Game/CustomContent/UGC2322974461/Blueprints/Gamemode/GamemodeStates` (`self.State`)
    (:`NewEnumerator0`
      (`self.HandleInit`))
    (:`NewEnumerator1`
      (`self.HandleLobby`))
    (:`NewEnumerator6`
      (`self.HandleGameStart`))
    (:`NewEnumerator2`
      (switch `/Game/CustomContent/UGC2322974461/Blueprints/Gamemode/RoundStates` (`self.RoundState`)
        (:`NewEnumerator0`
          (`self.HandlePlayersInit`))
        (:`NewEnumerator1`
          (`self.HandlePlayersSpawn`))
        (:`NewEnumerator2`
          (`self.HandleRoundInit`))
        (:`NewEnumerator3`
          (`self.HandleRoundMain`))))))

(fn `CreatePlayerTasksStruct`
  (params (Player :type "/Game/CustomContent/UGC2322974461/Blueprints/Player/RedIsSusPlayerBP Object Reference"))
  (returns (PlayerTask :type "/Game/CustomContent/UGC2322974461/Blueprints/Tasks/PlayerTasksStruct Structure"))
  (locals (ShortTasks :type Integer) (MediumTasks :type Integer) (LongTasks :type Integer) (CommonTasks :type Integer) (PlayerTasks :type "Array of /Game/CustomContent/UGC2322974461/Blueprints/Tasks/SpecificPlayerTaskStruct Structure"))
  (bind (_settings_imposteramount _settings_voicechatmode _settings_commontaskamount _settings_shorttaskamount _settings_mediumtaskamount _settings_longtaskamount) (break `/Game/CustomContent/UGC2322974461/Blueprints/Settings/SettingsStruct` (`self.Settings`)))
  (bind _tasks (`self.Tasks`))
  (`KismetArrayLibrary.Array_Shuffle` _tasks) ; Shuffle tasks so that this player gets unique tasks.
  (for _array_element _tasks
    (bind (_id _title _common _length _taskbp) (break `/Game/CustomContent/UGC2322974461/Blueprints/Tasks/BaseTask/TaskStruct` _array_element))
    (if _common
      ;[1 1 1] Add a common task
      (if (< (`local.CommonTasks`) _settings_commontaskamount)
        (`/Engine/EditorBlueprintResources/StandardMacros.IncrementInt` (`local.CommonTasks`)
          (:`  `
            (`KismetArrayLibrary.Array_Add` (`local.PlayerTasks`) (make `/Game/CustomContent/UGC2322974461/Blueprints/Tasks/SpecificPlayerTaskStruct` _array_element) :!label _label)
            (`/Game/CustomContent/UGC2322974461/Blueprints/Tasks/BaseTask/BaseTaskBP.SetCanBeCompleted` _taskbp (`KJModPlayerProxy.playerController` Player)))))
      (else
        (switch `/Game/CustomContent/UGC2322974461/Blueprints/Tasks/BaseTask/TaskLengthEnum` _length
          (:`NewEnumerator0`
            ;[1 1 1] Add Short task
            (if (< (`local.ShortTasks`) _settings_shorttaskamount)
              (`/Engine/EditorBlueprintResources/StandardMacros.IncrementInt` (`local.ShortTasks`)
                (:`  `
                  (goto _label)))))
          (:`NewEnumerator1`
            ;[1 1 1] Add medium task
            (if (< (`local.MediumTasks`) _settings_mediumtaskamount)
              (`/Engine/EditorBlueprintResources/StandardMacros.IncrementInt` (`local.MediumTasks`)
                (:`  `
                  (goto _label)))))
          (:`NewEnumerator2`
            ;[1 1 1] Add long task
            (if (< (`local.LongTasks`) _settings_longtaskamount)
              (`/Engine/EditorBlueprintResources/StandardMacros.IncrementInt` (`local.MediumTasks`)
                (:`  `
                  (goto _label)))))))))
  (return (make `/Game/CustomContent/UGC2322974461/Blueprints/Tasks/PlayerTasksStruct` Player (`local.PlayerTasks`))))

(fn `CreateSpawnPointList`
  (bind _outactors (`GameplayStatics.GetAllActorsWithTag` "SpawnPoint"))
  (set `self.SpawnPoints` _outactors))

(fn `FindNewServerLeader`
  (for _array_element (`self.Players`)
    (if (not (`/Game/CustomContent/UGC2322974461/Blueprints/Player/RedIsSusPlayerBP.IsServerLeader` _array_element))
      (set `/Game/CustomContent/UGC2322974461/Blueprints/Player/RedIsSusPlayerBP.IsServerLeader` true _array_element) ; Found first player who isnt leader
      (return))))

(fn `HandleGameStart`
  (for _array_element (`self.Players`)
    (`/Game/CustomContent/UGC2322974461/Blueprints/Player/RedIsSusPlayerBP.GameHasStartedServer` _array_element))
  (set `self.AliveCrewmateCount` 0)
  (set `self.AliveImpostorsCount` 0)
  (`self.InitalizeTasks`)
  (`self.SwitchToNewRoundState` "NewEnumerator0")
  (`self.SwitchToNewState` "NewEnumerator2"))

(fn `HandleInit`
  (`self.SwitchToNewState` "NewEnumerator1")
  (for _array_element (`self.Players`)
    (`self.SpawnPlayer` _array_element)))

(fn `HandleLobby`)

(fn `HandlePlayersInit`
  (bind _settings_imposteramount (break `/Game/CustomContent/UGC2322974461/Blueprints/Settings/SettingsStruct` (`self.Settings`)))
  (bind _shuffledplayers (`self.ShufflePlayers` (`self.Players`)))
  (for _array_element _shuffledplayers
    (if (< (`KismetArrayLibrary.Array_Length` (`self.Impostors`)) _settings_imposteramount)
      (set `/Game/CustomContent/UGC2322974461/Blueprints/Player/RedIsSusPlayerBP.IsImpostor` true _array_element) ; We dont have enough impostors yet
      (`/Engine/EditorBlueprintResources/StandardMacros.IncrementInt` (`self.AliveImpostorsCount`)
        (:`  `
          (`KismetArrayLibrary.Array_Add` (`self.Impostors`) _array_element)
          (`/Game/CustomContent/UGC2322974461/Blueprints/Player/RedIsSusPlayerBP.UpdateImpostorTaskList` _array_element (`self.Tasks`))))
      (else
        (set `/Game/CustomContent/UGC2322974461/Blueprints/Player/RedIsSusPlayerBP.IsImpostor` false _array_element) ; We have enough impostors.
        (bind _playertask (`self.CreatePlayerTasksStruct` _array_element))
        (`KismetArrayLibrary.Array_Add` (`self.PlayersWithTasks`) _playertask)
        (bind (_player _tasks) (break `/Game/CustomContent/UGC2322974461/Blueprints/Tasks/PlayerTasksStruct` _playertask))
        (`/Game/CustomContent/UGC2322974461/Blueprints/Player/RedIsSusPlayerBP.UpdateTaskList` _player _tasks)
        (`/Engine/EditorBlueprintResources/StandardMacros.IncrementInt` (`self.AliveCrewmateCount`)))))
  (`self.SwitchToNewRoundState` "NewEnumerator1"))

(fn `HandlePlayersSpawn`
  (locals (CurrentSpawnPoint :type Integer))
  (bind _output (`|GetArrayItem` (`self.SpawnPoints`) (`local.CurrentSpawnPoint`)))
  (bind _returnvalue (`self.K2_GetActorLocation` _output))
  (for _array_element (`self.Players`)
    (if (`KismetSystemLibrary.IsValid` _output)
      (`KismetSystemLibrary.PrintString` (`KismetStringLibrary.Conv_VectorToString` _returnvalue) true true (struct :`R` 1.0 :`B` 0.076772 :`A` 1.0) 15.0)
      (bind _playerpawn (`KJModPlayerProxy.playerPawn` _array_element))
      (`self.K2_SetActorLocation` _playerpawn _returnvalue false true)
      (`KismetSystemLibrary.PrintString` (`KismetStringLibrary.Concat_StrStr` (`KismetSystemLibrary.GetDisplayName` _playerpawn) (`KismetStringLibrary.Conv_VectorToString` (`self.K2_GetActorLocation` _playerpawn))) true true (struct :`R` 0.098742 :`B` 1.0 :`A` 1.0) 15.0)
      (bind _result (`/Engine/EditorBlueprintResources/StandardMacros.IncrementInt` (`local.CurrentSpawnPoint`))
        (:`  `
          (if (>= _result (`KismetArrayLibrary.Array_Length` (`self.SpawnPoints`)))
            (set `local.CurrentSpawnPoint` 0))))))
  (set `self.RoundState` "NewEnumerator2"))

(fn `HandleRoundInit`
  (for _array_element (`self.Players`)
    (`/Game/CustomContent/UGC2322974461/Blueprints/Player/RedIsSusPlayerBP.RoundInitServer` _array_element))
  (`self.SwitchToNewRoundState` "NewEnumerator3"))

(fn `HandleRoundMain`
  (if (not (<= (`self.AliveCrewmateCount`) (`self.AliveImpostorsCount`)))
    (if (not (not (<= (`self.AliveImpostorsCount`) 0)))
      (`KismetSystemLibrary.PrintString` "crewmates win"))
    (else
      (`KismetSystemLibrary.PrintString` "impostors win"))))

(fn `HandleRoundReset`
  (`self.SwitchToNewRoundState` "NewEnumerator0")
  (`self.SwitchToNewState` "NewEnumerator1"))

(fn `OnRep_RoundState`)

(fn `OnRep_State`)

(fn `PlayerHasJoined`
  (params (joiningPlayerController :type "PlayerController Object Reference"))
  (returns (ReturnValue :type "KJModPlayerProxy Object Reference"))
  (`/Engine/EditorBlueprintResources/StandardMacros.IncrementInt` (`self.CurrentPlayerCount`)
    (:`  `
      (`KismetSystemLibrary.PrintString` "player joined." true true (struct :`G` 1.0 :`B` 0.087257 :`A` 1.0) 10.0)
      (bind _returnvalue (`|SpawnActorFromClass` "/Game/CustomContent/UGC2322974461/Blueprints/Player/RedIsSusPlayerBP.RedIsSusPlayerBP_C" (`KismetMathLibrary.MakeTransform` (0.0 0.0 0.0)) "Undefined" "OverrideRootScale" joiningPlayerController false self null))
      ;[1 1 1] Save player and intialise it with controller.
      (`KismetArrayLibrary.Array_Add` (`self.Players`) _returnvalue)
      (`KJModPlayerProxy.Initialise` _returnvalue joiningPlayerController self (make `KJModPlayerProxyPawnSettings` 0 0 true true true))
      (if (not (> (`self.CurrentPlayerCount`) 1))
        (set `/Game/CustomContent/UGC2322974461/Blueprints/Player/RedIsSusPlayerBP.IsServerLeader` true _returnvalue) ; If only player on server, its the leader.
      )
      (switch `/Game/CustomContent/UGC2322974461/Blueprints/Gamemode/GamemodeStates` (`self.State`)
        (:`NewEnumerator1`
          (`self.SpawnPlayer` _returnvalue) ; If game is in lobby we spawn the player
        )
        (:`NewEnumerator2`
          (`/Game/CustomContent/UGC2322974461/Blueprints/Player/RedIsSusPlayerBP.GameHasStartedServer` _returnvalue)))
      (return _returnvalue))))

(fn `PlayerHasLeft`
  (params (leavingPlayerController :type "PlayerController Object Reference"))
  (returns (ReturnValue :type Boolean))
  (`/Engine/EditorBlueprintResources/StandardMacros.DecrementInt` (`self.CurrentPlayerCount`)
    (:`  `
      ;[1 1 1] Search all previously recorded player representations for a matching entry
      (for _array_element (`self.Players`)
        (if (== leavingPlayerController (`KJModPlayerProxy.playerController` _array_element))
          (if (`/Game/CustomContent/UGC2322974461/Blueprints/Player/RedIsSusPlayerBP.IsServerLeader` _array_element)
            (`self.FindNewServerLeader`) ; Player was leader so find a new one
          )
          ;[1 1 1] Destroy and remove..
          (`self.K2_DestroyActor` _array_element) ; Destroy it
          (`KismetArrayLibrary.Array_RemoveItem` (`self.Players`) _array_element) ; Remove from array
          (`KismetSystemLibrary.PrintString` "Player left" true true (struct :`R` 0.625 :`B` 0.087781 :`A` 1.0) 10.0)
          (return false))))))

(fn `ShufflePlayers`
  (params (Players :type "Array of /Game/CustomContent/UGC2322974461/Blueprints/Player/RedIsSusPlayerBP Object Reference"))
  (returns (ShuffledPlayers :type "Array of /Game/CustomContent/UGC2322974461/Blueprints/Player/RedIsSusPlayerBP Object Reference"))
  (locals (LocalPlayers :type "Array of /Game/CustomContent/UGC2322974461/Blueprints/Player/RedIsSusPlayerBP Object Reference"))
  (bind _output_get (set `local.LocalPlayers` Players))
  (`KismetArrayLibrary.Array_Shuffle` _output_get)
  (return (`local.LocalPlayers`)))

(fn `SwitchToNewRoundState`
  (params (RoundState :type "/Game/CustomContent/UGC2322974461/Blueprints/Gamemode/RoundStates Enum" :default "NewEnumerator0"))
  (bind _output_get (set `self.RoundState` RoundState))
  (`KismetSystemLibrary.PrintString` (`|GetEnumeratorNameAsString` _output_get) true true (struct :`G` 0.66 :`B` 1.0 :`A` 1.0) 10.0))

(fn `SwitchToNewState`
  (params (State :type "/Game/CustomContent/UGC2322974461/Blueprints/Gamemode/GamemodeStates Enum" :default "NewEnumerator0"))
  (bind _output_get (set `self.State` State))
  (`KismetSystemLibrary.PrintString` (`|GetEnumeratorNameAsString` _output_get) true true (struct :`G` 0.66 :`B` 1.0 :`A` 1.0) 10.0))

(fn `UserConstructionScript`)
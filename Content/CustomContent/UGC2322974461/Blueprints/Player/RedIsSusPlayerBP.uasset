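; Player proxy for the RedIsSus impostor game mode, handling per-player state, task UI and game start by the server leader.
; On init, the server removes tools and guns, while the local client creates leader, crew and impostor task widgets; on spawn, the proxy attaches to its pawn.
; Server-to-client events show the role's task list; Space toggles the leader menu pre-game.
; Box-overlap task activation exists but is not hooked up.
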(event `self.Initialised`
  (`/Game/CustomContent/UGC2322974461/Blueprints/Macros.HandleClientServerLogic`
    (:`ServerLogic`
      (`self.InitalizePlayerServer`))
    (:`ClientLogic`
      (`self.SetViewModes` "ThirdPerson")
      (`self.IsLocalOrRemote`
        (:`IsLocal`
          ;[1 1 1] So we can receive keys (like F4)
          (`self.EnableInput` (`GameplayStatics.GetPlayerController` 0))
          (bind _returnvalue (`|CreateWidget` "/Game/CustomContent/UGC2322974461/Blueprints/UI/LeaderWidgetBP.LeaderWidgetBP_C" (`GameplayStatics.GetPlayerController` 0) self))
          (set `self.LeaderWidgetBP` _returnvalue)
          (`self.SetInputMode` "GameFocused" _returnvalue) ; Set input mode to game focused
          (bind _returnvalue_2 (`|CreateWidget` "/Game/CustomContent/UGC2322974461/Blueprints/UI/TaskList/TaskListWidgetBP.TaskListWidgetBP_C" (`GameplayStatics.GetPlayerController` 0) self))
          (set `self.TaskListWidgetBP` _returnvalue_2)
          (bind _returnvalue_3 (`|CreateWidget` "/Game/CustomContent/UGC2322974461/Blueprints/UI/TaskList/ImpostorTaskListWidgetBP.ImpostorTaskListWidgetBP_C" (`GameplayStatics.GetPlayerController` 0) self))
          (set `self.ImpostorTaskListWidgetBP` _returnvalue_3))))))

(event `InitalizePlayerServer`
  ;[1 1 1] No guns or tools in this mode (or do we every "give" any)
  (`self.SetDefaultToolAndGunSettings` (make `KJModPlayerProxyDefaultToolAndGunSetting` "NoToolsOrGuns")))

(event `self.ReceiveBeginPlay`)

(event `self.PlayerSpawnedWithPawn`
  (`KismetSystemLibrary.PrintString` "PlayerProxy - Spawned with pawn called" true true (struct :`G` 0.66 :`B` 1.0 :`A` 1.0) 10.0)
  ;[1 1 1] Check if server
  (`/Game/CustomContent/UGC2322974461/Blueprints/Macros.HandleClientServerLogic`
    (:`ServerLogic`
      (`self.K2_AttachToActor` (`self.playerPawn`) "None" "SnapToTarget" "SnapToTarget" "SnapToTarget") ; Attach proxy to pawn so that positions are the same.
      (`self.K2_SetActorRelativeTransform` (`KismetMathLibrary.MakeTransform` (0.0 0.0 0.0)) false true) ; Lets make sure tha proxy is in the middle of the pawn.
      (`self.PlayerSpawnedClient`))))

(event `PlayerSpawnedClient`)

(event `GameHasStartedServer`
  (set `self.IsGameActive` true)
  (`KismetSystemLibrary.PrintString` "player : game has started")
  (`self.GameHasStartedClient`))

(event `GameHasStartedClient`)

(event `StartGameClient`
  (`self.StartGameServer`))

(event `StartGameServer`
  (if (`self.IsServerLeader`)
    (`/Game/CustomContent/UGC2322974461/Blueprints/Gamemode/RedIsSusGamemodeBP.SetSettings` (`self.Gamemode`) (make `/Game/CustomContent/UGC2322974461/Blueprints/Settings/SettingsStruct` 1))))

(event `RoundInitServer`
  (`self.RoundInitClient`))

(event `RoundInitClient`
  (if (`self.IsImpostor`)
    (`UserWidget.AddToViewport` (`self.ImpostorTaskListWidgetBP`) 2)
    (else
      (`UserWidget.AddToViewport` (`self.TaskListWidgetBP`) 2))))

(event `UpdateTaskList`
  (params (PlayerTasks :type "Array of /Game/CustomContent/UGC2322974461/Blueprints/Tasks/SpecificPlayerTaskStruct Structure"))
  (`/Game/CustomContent/UGC2322974461/Blueprints/UI/TaskList/TaskListWidgetBP.FillTasks` (`self.TaskListWidgetBP`) PlayerTasks))

(event `UpdateImpostorTaskList`
  (params (AllTasks :type "Array of /Game/CustomContent/UGC2322974461/Blueprints/Tasks/BaseTask/TaskStruct Structure"))
  (`/Game/CustomContent/UGC2322974461/Blueprints/UI/TaskList/ImpostorTaskListWidgetBP.FillTasks` (`self.ImpostorTaskListWidgetBP`) AllTasks))

(event `Key|SpaceBar`
  (params (Key :type "Key Structure"))
  (:`Released`
    (`/Game/CustomContent/UGC2322974461/Blueprints/Macros.HandleClientServerLogic`
      (:`ClientLogic`
        (if (and (not (`self.IsGameActive`)) (`self.IsServerLeader`))
          (`/Game/CustomContent/UGC2322974461/Blueprints/UI/LeaderWidgetBP.ToggleLeaderWidget` (`self.LeaderWidgetBP`))
          (elif (not (`self.IsImpostor`))
            _))))))

(event `LookForTaskToUseClient`
  (bind _box (`self.Box`))
  (bind (_outactors _returnvalue) (`KismetSystemLibrary.ComponentOverlapActors` _box (`SceneComponent.K2_GetComponentToWorld` _box) (`|MakeArray` "ObjectTypeQuery1" "ObjectTypeQuery2" "ObjectTypeQuery4" :!type "EObjectTypeQuery Enum")))
  (if _returnvalue
    (for _array_element _outactors
      (if (`KismetSystemLibrary.DoesImplementInterface` _array_element "/Game/CustomContent/UGC2322974461/Blueprints/Tasks/BaseTask/TaskInterfaceBP.TaskInterfaceBP_C")
        (message `/Game/CustomContent/UGC2322974461/Blueprints/Tasks/BaseTask/TaskInterfaceBP.ActivateTask` _array_element)
        (break)))))

(event `LookForTaskToUseServer`)

(fn `OnRep_IsGameActive`)

(fn `OnRep_IsImpostor`)

(fn `OnRep_IsServerLeader`)

(fn `UserConstructionScript`)
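; TestTaskBP is a custom-content test task that registers itself on BeginPlay as a common task titled "Test Place: Test task".
; ActivateTaskClient runs ActivateWidget on the client-logic branch, creating TestTaskWidgetBP, adding it to the viewport and passing it a reference to the task.
; Destroying the task removes the widget if still valid.
; ActivateTask is empty, so the task's only behavior here is showing that widget.
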(event `self.ReceiveBeginPlay`
  (`parent.ReceiveBeginPlay`)
  (`self.SetTaskInformation` true "NewEnumerator0" "Test Place: Test task"))

(event `/Game/CustomContent/UGC2322974461/Blueprints/Tasks/TaskInterfaceBP.ActivateTask`)

(event `ActivateWidget`
  (bind _returnvalue (`|CreateWidget` "/Game/CustomContent/UGC2322974461/Blueprints/Tasks/TestTask/TestTaskWidgetBP.TestTaskWidgetBP_C"))
  (set `self.TaskWidgetBP` _returnvalue)
  (`UserWidget.AddToViewport` _returnvalue 5)
  (set `/Game/CustomContent/UGC2322974461/Blueprints/Tasks/TestTask/TestTaskWidgetBP.TaskBP` self _returnvalue)
  (`KismetSystemLibrary.PrintString` "Activated task"))

(event `self.ActivateTaskClient`
  (`/Game/CustomContent/UGC2322974461/Blueprints/Macros.HandleClientServerLogic`
    (:`ClientLogic`
      (`self.ActivateWidget`))))

(event `self.ReceiveDestroyed`
  (`self.RemoveWidget`))

(event `RemoveWidget`
  (bind _taskwidgetbp (`self.TaskWidgetBP`))
  (if (`KismetSystemLibrary.IsValid` _taskwidgetbp)
    (`Widget.RemoveFromParent` _taskwidgetbp)))

(fn `UserConstructionScript`
  (`parent.UserConstructionScript`))
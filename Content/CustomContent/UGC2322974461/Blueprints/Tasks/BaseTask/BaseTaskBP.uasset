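; BaseTaskBP is a base task actor that stores a title, length and common-task setting, apparently for player-completable tasks.
; SetCanBeCompleted runs client logic that highlights the actor yellow and flags it as completable.
; CompleteTask forwards to a server-logic event that only prints the gamemode name so far.
; Input is enabled for player 0 on BeginPlay, and releasing Space prints debug text without checking the flag or completing the task.
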(event `self.ReceiveBeginPlay`
  (`self.EnableInput` (`GameplayStatics.GetPlayerController` 0)))

(event `SetTaskInformation`
  (params (CommonTask :type Boolean) (Length :type "/Game/CustomContent/UGC2322974461/Blueprints/Tasks/BaseTask/TaskLengthEnum Enum" :default "NewEnumerator0") (Title :type String))
  (set `self.CommonTask` CommonTask)
  (set `self.Length` Length)
  (set `self.Title` Title))

(event `SetCanBeCompleted`
  (params (`Player Controller` :type "PlayerController Object Reference"))
  (`/Game/CustomContent/UGC2322974461/Blueprints/Macros.HandleClientServerLogic`
    (:`ClientLogic`
      (`KJModUtilityActor.AddObjectHighlight` `Player Controller` self "Yellow")
      (set `self.ClientCanComplete` true))))

(event `/Game/CustomContent/UGC2322974461/Blueprints/Tasks/BaseTask/TaskInterfaceBP.CompleteTask`
  (`self.EventCompleteTaskServer`))

(event `EventCompleteTaskServer`
  (`/Game/CustomContent/UGC2322974461/Blueprints/Macros.HandleClientServerLogic`
    (:`ServerLogic`
      (`KismetSystemLibrary.PrintString` (`KismetSystemLibrary.GetDisplayName` (`self.GamemodeBP`))))))

(event `Key|SpaceBar`
  (params (Key :type "Key Structure"))
  (:`Released`
    (`KismetSystemLibrary.PrintString` "pressed space next to task.")
    (`KismetSystemLibrary.PrintString` (`KismetSystemLibrary.GetDisplayName` (`self.GetOwner`)))))

(fn `UserConstructionScript`)
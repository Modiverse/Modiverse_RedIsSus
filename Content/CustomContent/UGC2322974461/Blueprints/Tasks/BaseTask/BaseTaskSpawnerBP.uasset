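; Base spawner for tasks in an impostor-style game mode, placed in the world and highlighted yellow for players assigned its task.
; On the server, an assigned non-impostor player overlapping the mesh gets their own task actor, of the class from GetTaskInformation, linked to the spawner and TaskId.
; Ending overlap destroys that player's task actor, found by owner.
; Two player lists track assignments and active spawns; completion clears the assignment.
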(event `self.SpawnerMesh.OnComponentBeginOverlap`
  (params (OverlappedComponent :type "PrimitiveComponent Object Reference") (OtherActor :type "Actor Object Reference") (OtherComp :type "PrimitiveComponent Object Reference") (OtherBodyIndex :type Integer) (bFromSweep :type Boolean) (SweepResult :type "HitResult Structure (by ref)"))
  (`/Game/CustomContent/UGC2322974461/Blueprints/Macros.HandleClientServerLogic`
    (:`ServerLogic`
      (bind _askjmod_player_proxy (cast `KJModPlayerProxy` OtherActor))
      (if (`self.ActorHasTag` _askjmod_player_proxy "Impostor")
        _
        (elif (>= (`KismetArrayLibrary.Array_Find` (`self.PlayersHasTask`) _askjmod_player_proxy) 0)
          (`self.CreateTaskBPServer` _askjmod_player_proxy))))))

(event `CreateTaskBPServer`
  (params (OverlappingPlayerProxy :type "KJModPlayerProxy Object Reference"))
  (if (< (`KismetArrayLibrary.Array_Find` (`self.PlayersSpawnedTask`) OverlappingPlayerProxy) 0)
    (bind (_title _common _length _taskclass) (`/Game/CustomContent/UGC2322974461/Blueprints/Tasks/SpawnerTaskInterfaceBP.GetTaskInformation`))
    (bind _returnvalue (`|SpawnActorFromClass` _taskclass (`self.GetTransform`) "AlwaysSpawn" "OverrideRootScale" OverlappingPlayerProxy null))
    (bind _asbase_task_bp (cast `/Game/CustomContent/UGC2322974461/Blueprints/Tasks/BaseTask/BaseTaskBP` _returnvalue))
    (set `/Game/CustomContent/UGC2322974461/Blueprints/Tasks/BaseTask/BaseTaskBP.TaskId` (`self.TaskId`) _asbase_task_bp)
    (set `/Game/CustomContent/UGC2322974461/Blueprints/Tasks/BaseTask/BaseTaskBP.Spawner` self _asbase_task_bp)
    (`KismetArrayLibrary.Array_Add` (`self.PlayersSpawnedTask`) OverlappingPlayerProxy)))

(event `self.SpawnerMesh.OnComponentEndOverlap`
  (params (OverlappedComponent :type "PrimitiveComponent Object Reference") (OtherActor :type "Actor Object Reference") (OtherComp :type "PrimitiveComponent Object Reference") (OtherBodyIndex :type Integer))
  (`/Game/CustomContent/UGC2322974461/Blueprints/Macros.HandleClientServerLogic`
    (:`ServerLogic`
      (bind _askjmod_player_proxy (cast `KJModPlayerProxy` OtherActor))
      (bind (_title _common _length _taskclass) (`/Game/CustomContent/UGC2322974461/Blueprints/Tasks/SpawnerTaskInterfaceBP.GetTaskInformation`))
      (bind _outactors (`GameplayStatics.GetAllActorsOfClass` _taskclass))
      (for _array_element _outactors
        (if (== _askjmod_player_proxy (`self.GetOwner` _array_element))
          (`KismetArrayLibrary.Array_RemoveItem` (`self.PlayersSpawnedTask`) _askjmod_player_proxy)
          (`self.K2_DestroyActor` _array_element))))))

(event `/Game/CustomContent/UGC2322974461/Blueprints/Tasks/SpawnerTaskInterfaceBP.SetCanBeCompleted`
  (params (CanComplete :type Boolean) (PlayerProxy :type "KJModPlayerProxy Object Reference"))
  (if CanComplete
    (`/Game/CustomContent/UGC2322974461/Blueprints/Macros.HandleClientServerLogic`
      (:`ServerLogic`
        (`self.SetCanBeCompletedServer` PlayerProxy)))))

(event `SetCanBeCompletedServer`
  (params (PlayerProxy :type "KJModPlayerProxy Object Reference"))
  (`KJModUtilityActor.AddObjectHighlight` (`KJModPlayerProxy.playerController` PlayerProxy) self "Yellow")
  (`KismetArrayLibrary.Array_Add` (`self.PlayersHasTask`) PlayerProxy))

(event `/Game/CustomContent/UGC2322974461/Blueprints/Tasks/SpawnerTaskInterfaceBP.SetTaskId`
  (params (TaskId :type Integer))
  (set `self.TaskId` TaskId))

(event `PlayerCompletedTaskServer`
  (params (Player :type "KJModPlayerProxy Object Reference"))
  (`/Game/CustomContent/UGC2322974461/Blueprints/Macros.HandleClientServerLogic`
    (:`ServerLogic`
      (`KismetArrayLibrary.Array_RemoveItem` (`self.PlayersHasTask`) Player))))

(fn `GetTaskId`
  (returns (TaskId :type Integer))
  (return (`self.TaskId`)))

(fn `GetTaskInformation`
  (returns (Title :type String) (Common :type Boolean) (Length :type "/Game/CustomContent/UGC2322974461/Blueprints/Tasks/TaskLengthEnum Enum") (TaskClass :type "Actor Class Reference"))
  (return "BaseTask that has stuff - wow task" true "NewEnumerator0" "/Game/CustomContent/UGC2322974461/Blueprints/Tasks/BaseTask/BaseTaskBP.BaseTaskBP_C"))

(fn `OnRep_TaskId`)

(fn `UserConstructionScript`)
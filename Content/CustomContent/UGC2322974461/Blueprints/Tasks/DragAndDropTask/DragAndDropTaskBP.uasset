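; DragAndDropTaskBP is a task Blueprint that opens the drag-and-drop task UI for a player.
; On client activation it creates DragAndDropWidgetBP, adds it to the viewport and passes itself to the widget.
; When its owner is a KJModPlayerProxy, it switches input focus to the widget to show the mouse.
; ActivateTask itself is empty, and no completion logic appears here.
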(event `/Game/CustomContent/UGC2322974461/Blueprints/Tasks/TaskInterfaceBP.ActivateTask`)

(event `ActivateWidget`
  (bind _returnvalue (`|CreateWidget` "/Game/CustomContent/UGC2322974461/Blueprints/Tasks/DragAndDropTask/DragAndDropWidgetBP.DragAndDropWidgetBP_C"))
  (set `self.TaskWidgetBP` _returnvalue)
  (`UserWidget.AddToViewport` _returnvalue 5)
  (bind _askjmod_player_proxy (cast `KJModPlayerProxy` (`self.GetOwner`))
    (:`then`
      (`KJModPlayerProxy.SetInputMode` _askjmod_player_proxy "UserInterfaceFocused" _returnvalue) ; Show mouse
    )
    (:`CastFailed`
      _))
  (set `/Game/CustomContent/UGC2322974461/Blueprints/Tasks/DragAndDropTask/DragAndDropWidgetBP.TaskBP` self _returnvalue)
  (`KismetSystemLibrary.PrintString` "Activated task"))

(event `self.ActivateTaskClient`
  (`/Game/CustomContent/UGC2322974461/Blueprints/Macros.HandleClientServerLogic`
    (:`ClientLogic`
      (`self.ActivateWidget`))))

(fn `UserConstructionScript`
  (`parent.UserConstructionScript`))
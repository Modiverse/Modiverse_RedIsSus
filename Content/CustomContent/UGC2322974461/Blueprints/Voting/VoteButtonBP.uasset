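; VoteButtonBP is a pawn-owned actor that lets the local player trigger a vote in the Red Is Sus game mode by releasing Space.
; While it exists, it shows the vote instruction on the owner's player proxy and hides it when destroyed.
; The key release passes through client and locally-controlled checks, then a client-to-server event pair calls TriggerVoteMessage with the owner on the first actor implementing RedIsSusGamemodeInterface.
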(event `self.ReceiveBeginPlay`
  (`/Game/CustomContent/UGC2322974461/Blueprints/Macros.IsLocallyControlled`
    (:`Locally`
      (`self.EnableInput` (`GameplayStatics.GetPlayerController` 0))
      ;[1 1 1] Set Space Instructions to vote
      (bind _aspawn (cast `Pawn` (`self.GetOwner`)))
      (bind _playerproxy (`/Game/CustomContent/UGC2322974461/Blueprints/Macros.FindPlayerProxyFromPawn` _aspawn)
        (:`Success`
          (message `/Game/CustomContent/UGC2322974461/Blueprints/Player/RedIsSusPlayerInterface.ShowVoteInstruction` _playerproxy))))))

(event `self.ReceiveDestroyed`
  (`/Game/CustomContent/UGC2322974461/Blueprints/Macros.IsLocallyControlled`
    (:`Locally`
      ;[1 1 1] Set space instructions to task
      (bind _aspawn (cast `Pawn` (`self.GetOwner`)))
      (bind _playerproxy (`/Game/CustomContent/UGC2322974461/Blueprints/Macros.FindPlayerProxyFromPawn` _aspawn)
        (:`Success`
          (message `/Game/CustomContent/UGC2322974461/Blueprints/Player/RedIsSusPlayerInterface.HideVoteInstruction` _playerproxy))))))

(event `Key|SpaceBar` :consume false
  (params (Key :type "Key Structure"))
  ;[1 1 1] ActivateVotingSession
  (:`Released`
    (`/Game/CustomContent/UGC2322974461/Blueprints/Macros.HandleClientServerLogic`
      (:`ClientLogic`
        (`/Game/CustomContent/UGC2322974461/Blueprints/Macros.IsLocallyControlled`
          (:`Locally`
            (`KismetSystemLibrary.PrintString` "pressed space next to vote.")
            (`KismetSystemLibrary.PrintString` "success")
            (`self.ActivateVoteClient`)))))))

(event `ActivateVoteClient`
  ;[1 1 1] ActivateVotingSession
  (`self.ActivateVoteServer`))

(event `ActivateVoteServer`
  ;[1 1 1] ActivateVotingSession
  (bind _outactors (`GameplayStatics.GetAllActorsWithInterface` "/Game/CustomContent/UGC2322974461/Blueprints/Gamemode/RedIsSusGamemodeInterface.RedIsSusGamemodeInterface_C"))
  (message `/Game/CustomContent/UGC2322974461/Blueprints/Gamemode/RedIsSusGamemodeInterface.TriggerVote` (`|GetArrayItem` _outactors) (`self.GetOwner`)))

(event `DeactivateVoteClient`)

(fn `UserConstructionScript`)
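; Voting trigger actor that gives each pawn entering its collision area a personal vote button.
; On the server, begin overlap spawns a VoteButtonBP at the actor's transform, owned by that pawn, and records the pawn to prevent duplicates.
; End overlap searches all VoteButtonBP actors for one owned by the leaving pawn, destroys it and removes the pawn from the list.
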(event `self.ReceiveBeginPlay`)

(event `self.ButtonCollision.OnComponentBeginOverlap`
  (params (OverlappedComponent :type "PrimitiveComponent Object Reference") (OtherActor :type "Actor Object Reference") (OtherComp :type "PrimitiveComponent Object Reference") (OtherBodyIndex :type Integer) (bFromSweep :type Boolean) (SweepResult :type "HitResult Structure (by ref)"))
  (`/Game/CustomContent/UGC2322974461/Blueprints/Macros.HandleClientServerLogic`
    (:`ServerLogic`
      (bind _aspawn (cast `Pawn` OtherActor))
      (if (< (`KismetArrayLibrary.Array_Find` (`self.PlayersSpawnedButton`) _aspawn) 0)
        (`|SpawnActorFromClass` "/Game/CustomContent/UGC2322974461/Blueprints/Voting/VoteButtonBP.VoteButtonBP_C" (`self.GetTransform`) "AlwaysSpawn" "OverrideRootScale" _aspawn null)
        (`KismetArrayLibrary.Array_Add` (`self.PlayersSpawnedButton`) _aspawn)))))

(event `self.ButtonCollision.OnComponentEndOverlap`
  (params (OverlappedComponent :type "PrimitiveComponent Object Reference") (OtherActor :type "Actor Object Reference") (OtherComp :type "PrimitiveComponent Object Reference") (OtherBodyIndex :type Integer))
  (`/Game/CustomContent/UGC2322974461/Blueprints/Macros.HandleClientServerLogic`
    (:`ServerLogic`
      (bind _aspawn (cast `Pawn` OtherActor))
      (bind _outactors (`GameplayStatics.GetAllActorsOfClass` "/Game/CustomContent/UGC2322974461/Blueprints/Voting/VoteButtonBP.VoteButtonBP_C"))
      (for _array_element _outactors
        (if (== _aspawn (`self.GetOwner` _array_element))
          (`KismetArrayLibrary.Array_RemoveItem` (`self.PlayersSpawnedButton`) _aspawn)
          (`self.K2_DestroyActor` _array_element)
          (break))))))

(fn `UserConstructionScript`)